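; BP_CoinCollector is a trigger actor that reports quest objective progress, apparently for testing the quest system.
; Any actor overlap casts the game state to BP_QuestGameState and calls ReportGameplayObjective with the configured type and target ID, amount one.
; The construction script labels its TextRender with that type and target, so each placed instance shows what it reports.
; It neither filters the overlapping actor nor removes itself afterward.
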(event `self.ReceiveActorBeginOverlap`
  (params (OtherActor :type "Actor Object Reference"))
  (bind _asbp_quest_game_state (cast `/Game/BPSystem/BP_QuestGameState` (`GameplayStatics.GetGameState`)))
  (`/Game/BPSystem/BP_QuestGameState.ReportGameplayObjective` _asbp_quest_game_state (`self.ObjetiveTestType`) (`self.ObjetiveTestID`) 1))

(fn `UserConstructionScript`
  (`TextRenderComponent.K2_SetText` (`self.TextRender`) (`|FormatText` "{Type} {Target}" (select `/Game/BPSystem/E_QuestObjectiveType` (`self.ObjetiveTestType`) :`NewEnumerator0` "kill" :`NewEnumerator1` "collect" :`NewEnumerator2` "interact" :`NewEnumerator3` "location" :!type "Text") (`self.ObjetiveTestID`))))