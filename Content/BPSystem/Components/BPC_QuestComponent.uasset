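; Quest component that tracks the runtime state, objective progress and completion of quests added from quest definitions, ignoring duplicate quest IDs.
; On BeginPlay it plays a 2D sound and binds to the BP_QuestGameState gameplay objective event, matching events by type and target ID against objectives in active quests.
; Matches add progress capped at the required amount, then trigger a completion check; start, progress and completion are broadcast through event dispatchers.
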(event `self.ReceiveBeginPlay`
  (bind _asbp_quest_game_state (cast `/Game/BPSystem/BP_QuestGameState` (`GameplayStatics.GetGameState`)))
  (add `/Game/BPSystem/BP_QuestGameState.OnGameplayObjectiveEvent` _asbp_quest_game_state (delegate `HandleGameplayObjective`))
  (`GameplayStatics.PlaySound2D` null 1.0 1.0 0.0 null null))

(event `HandleGameplayObjective`
  (params (ObjectiveType :type "/Game/BPSystem/E_QuestObjectiveType Enum" :default "NewEnumerator0") (TargetID :type Name) (Amount :type Integer))
  (for (_array_element _array_index) (`self.ActiveQuest`)
    (bind (_questid _questdefinition _objetives _isactive _iscompleted) (break `/Game/BPSystem/Structs/S_QuestRuntime` _array_element))
    (if (and _isactive (not _iscompleted))
      (for (_array_element_2 _array_index_2) _objetives
        (bind (_objetiveid _objetivetype _targetid) (break `/Game/BPSystem/Structs/S_QuestObjective` _array_element_2))
        (if (and (`|EnumEquality` _objetivetype ObjectiveType) (== _targetid TargetID))
          (`self.UpdateObjectiveProgress` _array_index _array_index_2 Amount))))))

(fn `AddQuest`
  (params (QuestDefinition :type "/Game/BPSystem/QuestData/PDA_QuestDefinition Object Reference"))
  (bind _s_questruntime (make `/Game/BPSystem/Structs/S_QuestRuntime` (`/Game/BPSystem/QuestData/PDA_QuestDefinition.QuestID` QuestDefinition) QuestDefinition (`/Game/BPSystem/QuestData/PDA_QuestDefinition.Objetives` QuestDefinition) true))
  (bind _found (`self.FindQuestByID` (`/Game/BPSystem/QuestData/PDA_QuestDefinition.QuestID` QuestDefinition)))
  (if (not _found)
    (`KismetArrayLibrary.Array_Add` (`self.ActiveQuest`) _s_questruntime)
    (`self.OnQuestStarted` _s_questruntime)))

(fn `CheckQuestCompleted`
  (params (QuestIndex :type Integer))
  (locals (HasIncompleteObjectives :type Boolean) (CurrentQuest :type "/Game/BPSystem/Structs/S_QuestRuntime Structure"))
  (bind _output (`|GetArrayItem` (`self.ActiveQuest`) QuestIndex))
  (set `local.CurrentQuest` _output)
  (set `local.HasIncompleteObjectives` false)
  (for _array_element (`.Objetives_27_4E4AA57A49741198A6E154A39A506A9B` (break `/Game/BPSystem/Structs/S_QuestRuntime` _output))
    (bind (_objetiveid _objetivetype _targetid _requiredamount _currentamount) (break `/Game/BPSystem/Structs/S_QuestObjective` _array_element))
    (if (not (>= _currentamount _requiredamount))
      (set `local.HasIncompleteObjectives` true)
      (break)))
  (if (not (`local.HasIncompleteObjectives`))
    (bind _structout (setmembers `/Game/BPSystem/Structs/S_QuestRuntime` :`StructRef` (`local.CurrentQuest`) :`IsActive` false :`IsCompleted` true))
    (`KismetArrayLibrary.Array_Set` (`self.ActiveQuest`) (`local.QuestIndex`) _structout)
    (`self.OnQuestCompleted` _structout)))

(fn `FindQuestByID`
  (params (QuestID :type Name))
  (returns (Found :type Boolean) (QuestData :type "/Game/BPSystem/Structs/S_QuestRuntime Structure") (QuestIndex :type Integer))
  (for (_array_element _array_index) (`self.ActiveQuest`)
    (if (== (`local.QuestID`) (`.QuestID_14_D83EAEBF4446BF7D8F3783B47881546A` (break `/Game/BPSystem/Structs/S_QuestRuntime` _array_element)))
      (return true _array_element _array_index)))
  (return false (struct) -1))

(fn `UpdateObjectiveProgress`
  (params (`QuestIndex ` :type Integer) (ObjectiveIndex :type Integer) (Amount :type Integer))
  (locals (ObjetiveResult :type "/Game/BPSystem/Structs/S_QuestObjective Structure"))
  (bind _output (`|GetArrayItem` (`.Objetives_27_4E4AA57A49741198A6E154A39A506A9B` (break `/Game/BPSystem/Structs/S_QuestRuntime` (`|GetArrayItem` (`self.ActiveQuest`) (`local.QuestIndex `)))) (`local.ObjectiveIndex`)))
  (bind (_objetiveid _objetivetype _targetid _requiredamount _currentamount) (break `/Game/BPSystem/Structs/S_QuestObjective` _output))
  (bind _structout (setmembers `/Game/BPSystem/Structs/S_QuestObjective` :`StructRef` _output :`CurrentAmount` (`KismetMathLibrary.Min` _requiredamount (+ _currentamount Amount))))
  (set `local.ObjetiveResult` _structout)
  (`self.OnQuestProgressChanged` (`|GetArrayItem` (`self.ActiveQuest`) (`local.QuestIndex `)))
  (`self.CheckQuestCompleted` (`local.QuestIndex `)))